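; BP_WaltherGun is a hitscan gun that damages BP_Zombie enemies.
; shootGun spends a round, attaches a Niagara muzzle flash and line traces forward from MuzzleLocation, spawning blood and applying damage on zombie hits.
; ReloadGun refills CurrentAmmo after a short delay, with IsReloading blocking shots and repeat reloads meanwhile.
; Debug trace drawing and print strings remain in the firing and reload logic.
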(event Custom|shootGun
  (bind _muzzlelocation (Variables|Default|GetMuzzleLocation))
  (bind _currentammo (Variables|Default|GetcurrentAmmo))
  (bind _muzzlelocation_2 (Variables|Default|GetMuzzleLocation))
  (bind _returnvalue (Transformation|GetWorldLocation _muzzlelocation))
  (bind _returnvalue_2 (Transformation|GetWorldRotation _muzzlelocation_2))
  ;[0.15 0.15 0.15 0.5] checks if player can shoot
  (if (not (Variables|Default|GetisReloading))
    (if (> _currentammo 0)
      (Math|Integer|DecrementInt _currentammo
        (:%20%20
          (Development|PrintString (Utilities|String|ToString(Integer) _currentammo))
          (Niagara|SpawnSystemAttached "/Game/test/fx/NS_Muzzleflash.NS_Muzzleflash" _muzzlelocation_2 "None" (+ (Transformation|GetWorldLocation _muzzlelocation_2) (* (Math|Vector|GetForwardVector _returnvalue_2) 3.0)) _returnvalue_2 "KeepWorldPosition" true true "AutoRelease")
          ;[0.15 0.15 0.15 0.5] spawns and cheks if raytrace hit a zombie
          (bind (_outhit _returnvalue_3) (Collision|LineTraceByChannel _returnvalue (+ _returnvalue (* (Math|Vector|GetForwardVector _muzzlelocation) 1e+04)) "TraceTypeQuery1" false 0 "ForDuration"))
          (if _returnvalue_3
            (Utilities|IsValid (.HitActor (Collision|BreakHitResult _outhit))
              (:Is%20Valid
                (Development|PrintString (Utilities|GetDisplayName (.HitActor (Collision|BreakHitResult _outhit))))
                (bind _asbp_zombie (Utilities|Casting|CastToBP_Zombie (.HitActor (Collision|BreakHitResult _outhit))))
                (Effects|SpawnEmitteratLocation "/Game/Realistic_Starter_VFX_Pack_Vol2/Particles/Blood/P_Blood_Splat_Cone.P_Blood_Splat_Cone" (.Location (Collision|BreakHitResult _outhit)) (Math|Rotator|Delta(Rotator) (Math|Conversions|RotationFromXVector (.Normal (Collision|BreakHitResult _outhit))) "90.000000,0.000000,0.000000") "0.500000,0.500000,0.500000")
                (Game|Damage|ApplyDamage _asbp_zombie 2e+01 0 (Game|GetPlayerCharacter 0))
                (Development|PrintString "Applied damage I think?")))))))))

(event Custom|Reload%20Gun
  (if (not (Variables|Default|GetisReloading))
    (Variables|Default|SetisReloading true)
    (Utilities|FlowControl|Delay 2.0)
    (bind _output_get (Variables|Default|SetcurrentAmmo 10))
    (Development|PrintString (Utilities|String|ToString(Integer) _output_get))
    (Variables|Default|SetisReloading false)))

(event EventBeginPlay)

(event Collision|EventActorBeginOverlap
  (params (OtherActor :type Actor%20Object%20Reference)))

(event EventTick
  (params (DeltaSeconds :type Float%20%28single-precision%29)))

(fn ConstructionScript)