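; Zombie enemy character for a round-based game that attacks the bean player and reports its death to MyZombieGameMode.
; While the player overlaps AttackRange, a looping one-second timer calls the player's TakeDamage.
; AnyDamage reduces ZombieHP, and at zero the game mode's active count drops and it checks for round end.
; Death also stops AI movement and logic, ragdolls the mesh, disables collision and destroys the actor after a delay.
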(event EventBeginPlay)

(event Collision|EventActorBeginOverlap
  (params (OtherActor :type Actor%20Object%20Reference)))

(event EventTick
  (params (DeltaSeconds :type Float%20%28single-precision%29)))

(event Game|Damage|EventAnyDamage
  (params (Damage :type Float%20%28single-precision%29) (DamageType :type Damage%20Type%20Object%20Reference) (InstigatedBy :type Controller%20Object%20Reference) (DamageCauser :type Actor%20Object%20Reference))
  (Development|PrintString (Utilities|GetDisplayName DamageType))
  (Development|PrintString (Utilities|String|ToString(Float) Damage))
  (CallFunction|TakeDamage Damage 0 DamageType))

(event OnComponentBeginOverlap(attackRange)
  (params (OverlappedComponent :type Primitive%20Component%20Object%20Reference) (OtherActor :type Actor%20Object%20Reference) (OtherComp :type Primitive%20Component%20Object%20Reference) (OtherBodyIndex :type Integer) (bFromSweep :type Boolean) (SweepResult :type Hit%20Result%20Structure%20%28by%20ref%29))
  ;[0.15 0.15 0.15 0.5] Attacks the player after 1 second
  (Utilities|Casting|CastToBP_beanPlayerCharacter OtherActor)
  (Development|PrintString "player entered")
  (Variables|Default|SetisPlayerInRange true)
  (bind _returnvalue (Utilities|Time|SetTimerbyFunctionName 0 "ReadyToAttack" 1.0 true))
  (Variables|Default|SetzombieTimerHandle _returnvalue))

(event OnComponentEndOverlap(attackRange)
  (params (OverlappedComponent :type Primitive%20Component%20Object%20Reference) (OtherActor :type Actor%20Object%20Reference) (OtherComp :type Primitive%20Component%20Object%20Reference) (OtherBodyIndex :type Integer))
  ;[0.15 0.15 0.15 0.5] timer resets when the player leaves the area
  (Utilities|Casting|CastToBP_beanPlayerCharacter OtherActor)
  (Development|PrintString "player left")
  (Utilities|Time|ClearandInvalidateTimerbyHandle (Variables|Default|GetzombieTimerHandle))
  (Variables|Default|SetisPlayerInRange false))

(fn ConstructionScript)

(fn TakeDamage
  (params (damageAmount :type Float%20%28double-precision%29) (instigator :type Actor%20Object%20Reference) (damageType :type Damage%20Type%20Object%20Reference))
  (Development|PrintString (Utilities|String|ToString(Float) (Variables|Default|GetzombieHP)))
  (Development|PrintString (Utilities|String|ToString(Float) damageAmount))
  (bind _output_get (Variables|Default|SetzombieHP (- (Variables|Default|GetzombieHP) damageAmount)))
  (if (<= _output_get 0.0)
    (CallFunction|HandleDeath)))

(fn HandleDeath
  (bind _returnvalue (Pawn|GetController))
  (bind _mesh (Variables|Character|GetMesh))
  (bind _returnvalue_2 (AI|GetAIController _returnvalue))
  (bind _asmy_zombie_game_mode (Utilities|Casting|CastToMyZombieGameMode (Game|GetGameMode)))
  (Variables|/Game/test/zombie/MyZombieGameMode.MyZombieGameMode_C|SetactiveZombiesCount _asmy_zombie_game_mode (- (Variables|/Game/test/zombie/MyZombieGameMode.MyZombieGameMode_C|GetactiveZombiesCount _asmy_zombie_game_mode) 1))
  (Default|CheckforRoundEnd _asmy_zombie_game_mode)
  (AI|Navigation|StopMovement _returnvalue_2)
  (Input|DisableInput 0)
  (AI|Logic|StopLogic (Variables|/Script/AIModule.AIController|GetBrainComponent _returnvalue_2) "")
  (Physics|SetSimulatePhysics _mesh true)
  (Collision|SetCollisionEnabled _mesh "PhysicsOnly")
  (Collision|SetCollisionEnabled (Variables|Collision|GetCapsuleComponent) "NoCollision")
  (Collision|SetCollisionEnabled (Variables|Default|GetattackRange) "NoCollision")
  (bind _returnvalue_3 (Utilities|Time|SetTimerbyFunctionName 0 "DestroyZombie" 5.0))
  (Variables|Default|SetdestroyZombieTimerHandle _returnvalue_3))

(fn ReadytoAttack
  (if (Variables|Default|GetisPlayerInRange)
    (bind _asbp_bean_player_character (Utilities|Casting|CastToBP_beanPlayerCharacter (Game|GetPlayerCharacter 0)))
    (Default|TakeDamage _asbp_bean_player_character)))

(fn DestroyZombie
  (Actor|DestroyActor)
  (Utilities|Time|ClearandInvalidateTimerbyHandle (Variables|Default|GetdestroyZombieTimerHandle)))