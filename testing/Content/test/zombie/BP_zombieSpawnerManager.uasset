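; Manager actor that spawns zombies for each round at random BP_ZombieSpawnPoint actors, which it gathers on BeginPlay.
; SpawnZombie spawns a BP_Zombie, increments the active and spawned-this-round counts on MyZombieGameMode, then schedules itself on a two-second timer.
; Each call clears that timer once any zombie has spawned, so spawning stops when the round's quota is reached.
; Nothing in this Blueprint makes the first SpawnZombie call.
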(event EventBeginPlay
  (bind _outactors (Actor|GetAllActorsOfClass "/Game/test/zombie/BP_ZombieSpawnPoint.BP_ZombieSpawnPoint_C"))
  (Variables|Default|SetspawnPoints _outactors))

(event Collision|EventActorBeginOverlap
  (params (OtherActor :type Actor%20Object%20Reference)))

(event EventTick
  (params (DeltaSeconds :type Float%20%28single-precision%29)))

(fn ConstructionScript)

(fn SpawnZombie
  (bind _asmy_zombie_game_mode (Utilities|Casting|CastToMyZombieGameMode (Game|GetGameMode)))
  (if (> (Variables|/Game/test/zombie/MyZombieGameMode.MyZombieGameMode_C|GetZombiesSpawnedThisRound _asmy_zombie_game_mode) 0)
    (Utilities|Time|ClearandInvalidateTimerbyHandle (Variables|Default|GetSpawnTimerHandler)))
  (if (not (== (Variables|/Game/test/zombie/MyZombieGameMode.MyZombieGameMode_C|GetZombiesSpawnedThisRound _asmy_zombie_game_mode) (Variables|/Game/test/zombie/MyZombieGameMode.MyZombieGameMode_C|GetzombiesPerRound _asmy_zombie_game_mode)))
    (Game|SpawnActorfromClass "/Game/test/zombie/BP_Zombie.BP_Zombie_C" (Math|Transform|MakeTransform (Transformation|GetActorLocation (Utilities|Array|Get(acopy) (Variables|Default|GetspawnPoints) (Math|Random|RandomIntegerinRange 0 (- (Utilities|Array|Length (Variables|Default|GetspawnPoints)) 1)))) "0, 0, 0" "1.000000,1.000000,1.000000") "AlwaysSpawn" "MultiplyWithRoot" 0 0)
    (bind _result (Math|Integer|IncrementInt (Variables|/Game/test/zombie/MyZombieGameMode.MyZombieGameMode_C|GetactiveZombiesCount _asmy_zombie_game_mode))
      (:%20%20
        (Variables|/Game/test/zombie/MyZombieGameMode.MyZombieGameMode_C|SetactiveZombiesCount _asmy_zombie_game_mode _result)
        (bind _result_2 (Math|Integer|IncrementInt (Variables|/Game/test/zombie/MyZombieGameMode.MyZombieGameMode_C|GetZombiesSpawnedThisRound _asmy_zombie_game_mode))
          (:%20%20
            (Variables|/Game/test/zombie/MyZombieGameMode.MyZombieGameMode_C|SetZombiesSpawnedThisRound _asmy_zombie_game_mode _result_2)
            (bind _returnvalue (Utilities|Time|SetTimerbyFunctionName 0 "SpawnZombie" 2.0 true))
            (Variables|Default|SetSpawnTimerHandler _returnvalue)))))))